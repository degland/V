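; BP_AISpawner_Waypointmet is an AI spawner that spawns AI when a payload reaches a configured waypoint.
; On BeginPlay it binds to the Payload's reached-target event if the Payload is valid.
; Each time that fires, it calls SpawnAI when the Payload's CurrentTarget equals Waypoint plus one, meaning the payload has just moved past that waypoint.
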(event `self.ReceiveBeginPlay`
  (bind _payload (`self.Payload`))
  (`/Engine/EditorBlueprintResources/StandardMacros.IsValid` _payload
    (:`Is Valid`
      (add `/Game/V/Payload/BP_Payload_Cart.OnPayloadReachedTarget` _payload (delegate `CheckSpawn`)))))

(event `CheckSpawn`
  (if (== (`/Game/V/Payload/BP_Payload_Cart.CurrentTarget` (`self.Payload`)) (+ (`self.Waypoint`) 1))
    (`self.SpawnAI`)))

(fn `UserConstructionScript`
  (`parent.UserConstructionScript`))