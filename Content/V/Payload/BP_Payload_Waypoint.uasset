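; Payload waypoint actor that plays a celebration when its OnCompleted event fires.
; The effect is skipped on dedicated servers.
; It plays a firework sound at its location, waits briefly, then spawns short-lived shooting star actors at four firework component transforms, followed by a cheer sound.
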(event `OnCompleted`
  (if (not (`KismetSystemLibrary.IsDedicatedServer`))
    (`GameplayStatics.PlaySoundAtLocation` "/Game/MarketplaceContent/BBC/firework.firework" (`self.K2_GetActorLocation`) (struct) 3.0 1.0 0.0 null null null)
    (`KismetSystemLibrary.Delay` 0.2)
    (for _index (range 4)
      (bind _returnvalue (`|SpawnActorFromClass` "/Game/FXVarietyPack/Blueprints/BP_ky_shootingStar1.BP_ky_shootingStar1_C" (`SceneComponent.K2_GetComponentToWorld` (select `int` _index :`0` (`self.firework`) :`1` (`self.firework1`) :`2` (`self.firework2`) :`3` (`self.firework3`))) "AlwaysSpawn" "OverrideRootScale" null null))
      (set `/Game/FXVarietyPack/Blueprints/BP_ky_shootingStar1.duration` 3.0 _returnvalue))
    (`GameplayStatics.PlaySoundAtLocation` "/Game/MarketplaceContent/BBC/cheer.cheer" (`self.K2_GetActorLocation`) (struct) 1.0 1.0 0.0 null null null)))

(fn `UserConstructionScript`)