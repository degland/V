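; Payload cart actor that players escort along waypoints while AI characters contest it or push it back.
; Each tick, sphere overlaps and waypoint blocking set its state, which drives segment progress, with advance speed scaling by pusher count.
; Position lerps between adjacent waypoints, so retreat stops at the last one reached.
; Completing waypoints advances the target until ticking stops; state changes fire an event and swap the status ring particles.
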(event `self.ReceiveBeginPlay`
  (`/Engine/EditorBlueprintResources/ActorMacros.Switch Has Authority`
    (:`Authority`
      (if (> (`KismetArrayLibrary.Array_Length` (`self.Waypoints`)) 0)
        (`self.K2_SetActorTransform` (`self.GetTransform` (`|GetArrayItem` (`self.Waypoints`))) false true)
        (else
          (`KismetSystemLibrary.PrintString` "No target points set in payload, deleting.")
          (`self.K2_DestroyActor`))))))

(event `self.ReceiveTick`
  (params (DeltaSeconds :type "Float (single-precision)"))
  (if (`self.CheckTargetValid`)
    (`self.UpdateState`)
    (`self.UpdateProgress`)
    (`self.UpdatePosition`)
    (`self.CheckTargetMet`)
    (else
      (set `self.CurrentState` "NewEnumerator4")
      (`self.SetActorTickEnabled` false))))

(fn `CheckTargetMet`
  (if (>= (`self.CurrentProgress`) 100.0)
    (`/Game/V/Payload/BP_Payload_Waypoint.OnCompleted` (`|GetArrayItem` (`self.Waypoints`) (`self.CurrentTarget`)))
    (`/Engine/EditorBlueprintResources/StandardMacros.IncrementInt` (`self.CurrentTarget`)
      (:`  `
        (set `self.CurrentProgress` 0.0)
        (`self.OnPayloadReachedTarget`)))))

(fn `CheckTargetValid`
  (returns (IsValid :type Boolean))
  (return (not (>= (`self.CurrentTarget`) (`KismetArrayLibrary.Array_Length` (`self.Waypoints`))))))

(fn `UpdateEmitter`
  (`ParticleSystemComponent.SetTemplate` (`self.StatusRing`) (select `/Game/V/Payload/E_Payload_State` (`self.CurrentState`) :`NewEnumerator0` "/Game/FXVarietyPack/Particles/P_ky_healAura_edit_green.P_ky_healAura_edit_green" :`NewEnumerator1` "/Game/FXVarietyPack/Particles/P_ky_healAura_edit_red.P_ky_healAura_edit_red" :`NewEnumerator2` "/Game/FXVarietyPack/Particles/P_ky_healAura_edit_red.P_ky_healAura_edit_red" :`NewEnumerator3` "/Game/FXVarietyPack/Particles/P_ky_healAura_edit_red.P_ky_healAura_edit_red" :`NewEnumerator4` "/Game/FXVarietyPack/Particles/P_ky_healAura_edit_green.P_ky_healAura_edit_green" :`NewEnumerator5` "/Game/FXVarietyPack/Particles/P_ky_healAura_edit_red.P_ky_healAura_edit_red" :!type "ParticleSystem Object Reference")))

(fn `UpdatePosition`
  (locals (NextLocation :type "Vector Structure" :default (0.0 0.0 0.0)) (PreviousLocation :type "Vector Structure" :default (0.0 0.0 0.0)))
  (`|ExecutionSequence`
    (:`then_0`
      (set `local.NextLocation` (`self.K2_GetActorLocation` (`|GetArrayItem` (`self.Waypoints`) (`self.CurrentTarget`))))
      (set `local.PreviousLocation` (`self.K2_GetActorLocation` (`|GetArrayItem` (`self.Waypoints`) (- (`self.CurrentTarget`) 1)))))
    (:`then_1`
      (`self.K2_SetActorLocation` (`KismetMathLibrary.VLerp` (`local.PreviousLocation`) (`local.NextLocation`) (/ (`self.CurrentProgress`) 100.0)) false true))))

(fn `UpdateProgress`
  (set `self.CurrentProgress` (`KismetMathLibrary.FClamp` (+ (`self.CurrentProgress`) (* (`GameplayStatics.GetWorldDeltaSeconds`) (select `/Game/V/Payload/E_Payload_State` (`self.CurrentState`) :`NewEnumerator0` (* (`self.CurrentPushingPlayers`) (`self.AdvanceRate`)) :`NewEnumerator2` (* -1 (`self.RetreatRate`))))) 0.0 100.0)))

(fn `UpdateState`
  (locals (OldState :type "/Game/V/Payload/E_Payload_State Enum" :default "NewEnumerator0"))
  (bind _returnvalue (`KismetArrayLibrary.Array_Length` (`PrimitiveComponent.GetOverlappingActors` (`self.Sphere`) "/Game/V/Player/BP_PlayerCharacter_Server.BP_PlayerCharacter_Server_C")))
  (set `local.OldState` (`self.CurrentState`))
  (`|ExecutionSequence`
    (:`then_0`
      (if (> (`KismetArrayLibrary.Array_Length` (`PrimitiveComponent.GetOverlappingActors` (`self.Sphere`) "/Game/V/AI/BP_AICharacterBase.BP_AICharacterBase_C")) 0)
        (if (== _returnvalue 0)
          (set `self.CurrentState` "NewEnumerator2")
          (else
            (set `self.CurrentState` "NewEnumerator5")))
        (elif (> _returnvalue 0)
          (if (`/Game/V/Payload/BP_Payload_Waypoint.Blocked` (`|GetArrayItem` (`self.Waypoints`) (`self.CurrentTarget`)))
            (set `self.CurrentState` "NewEnumerator3")
            (else
              (set `self.CurrentState` "NewEnumerator0")
              (set `self.CurrentPushingPlayers` _returnvalue)))
          (else
            (set `self.CurrentState` "NewEnumerator1")))))
    (:`then_1`
      (if (not (== (`local.OldState`) (`self.CurrentState`)))
        (`self.OnPayloadStateChanged`)
        (`self.UpdateEmitter`)))))

(fn `UserConstructionScript`)