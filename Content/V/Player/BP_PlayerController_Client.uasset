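; Player controller for cursor-driven play, splitting the client's camera pawn from a separately spawned server character and controller.
; On dedicated or listen servers, BeginPlay spawns that pair at a random PlayerStart; non-dedicated instances create the HUD.
; Held input sends cursor hit locations to the server controller's MoveToLocation, while Interact and Shoot forward to the server character.
; Tick eases the controlled pawn toward the server character as camera follow.
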(event `self.ReceivePossess`
  (params (PossessedPawn :type "Pawn Object Reference"))
  ;[1 1 1] Possess -> save the pawn so I can skip casting it repeatedly later
  (bind _asbp_player_pawn_client (cast `/Game/V/Player/BP_PlayerPawn_Client` PossessedPawn))
  (set `self.ClientPawn` _asbp_player_pawn_client))

(event `SetupServer`
  ;[1 1 1] Beginplay -> Setup server-side character & controller
  (bind _outactors (`GameplayStatics.GetAllActorsOfClass` "/Script/Engine.PlayerStart"))
  (bind _returnvalue (`self.GetTransform` (`KismetArrayLibrary.Array_Random` _outactors)))
  (bind _returnvalue_2 (`|SpawnActorFromClass` "/Game/V/Player/BP_PlayerCharacter_Server.BP_PlayerCharacter_Server_C" _returnvalue "Undefined" "OverrideRootScale" self null))
  (set `self.ServerCharacter` _returnvalue_2)
  (bind _returnvalue_3 (`|SpawnActorFromClass` "/Game/V/Player/BP_PlayerController_Server.BP_PlayerController_Server_C" _returnvalue "Undefined" "OverrideRootScale" self null))
  (set `self.ServerController` _returnvalue_3)
  (`self.Possess` (`self.ServerController`) (`self.ServerCharacter`)))

(event `self.ReceiveBeginPlay`
  ;[1 1 1] Beginplay -> Setup server-side character & controller
  (if (not (`KismetSystemLibrary.IsDedicatedServer`))
    (bind _returnvalue (`|CreateWidget` "/Game/V/UI/WBP_HUD.WBP_HUD_C" self))
    (bind _output_get (set `self.HUD` _returnvalue))
    (`UserWidget.AddToViewport` _output_get 0)
    (`/Engine/EditorBlueprintResources/ActorMacros.Switch Has Authority` ; If we're a listen server, we still want to do setup
      (:`Authority`
        _)))
  (`self.SetupServer`))

(event `MoveServerCharacter`
  (params (Target :type "Vector Structure"))
  (bind _servercontroller (`self.ServerController`))
  ;[1 1 1] Tick -> Move camera & server controller
  (`/Engine/EditorBlueprintResources/StandardMacros.IsValid` _servercontroller
    (:`Is Valid`
      (`AIController.MoveToLocation` _servercontroller Target -1.0 false true false true null true))))

(event `self.ReceiveTick`
  (params (DeltaSeconds :type "Float (single-precision)"))
  ;[1 1 1] Tick -> Move camera & server controller
  (`self.UpdateCameraPosition`)
  (`/Engine/EditorBlueprintResources/StandardMacros.Gate` true :!label _label ; While key is pressed...
    (:`Exit`
      (if (not (`self.BlockMovement`))
        (`self.MoveServerCharacter` (`.Location` (`GameplayStatics.BreakHitResult` (`self.GetHitResultUnderCursorByChannel` "TraceTypeQuery1")))) ; Okay it's not entirely client-only but at least if we get this far we have player input to handle
      ))))

(event `InputAction|SetDestination`
  (params (Key :type "Key Structure"))
  ;[1 1 1] Tick -> Move camera & server controller
  (:`Pressed`
    (goto _label :!via `Open`))
  (:`Released`
    (goto _label :!via `Close`)))

(event `InputAction|Interact`
  (params (Key :type "Key Structure"))
  ;[1 1 1] Interact
  (:`Pressed`
    (`self.ServerTryInteract`)))

(event `ServerTryInteract`
  ;[1 1 1] Interact
  (`/Game/V/Player/BP_InteractionComponent.DoInteract` (`/Game/V/Player/BP_PlayerCharacter_Server.InteractionComponent` (`self.ServerCharacter`))))

(event `ServerTryShoot`
  (params (Target :type "Vector Structure"))
  ;[1 1 1] Shoot projectile
  (`/Game/V/Player/BP_PlayerCharacter_Server.DoShoot` (`self.ServerCharacter`) Target))

(event `InputAction|Shoot`
  (params (Key :type "Key Structure"))
  ;[1 1 1] Shoot projectile
  (:`Pressed`
    (`self.ServerTryShoot` (`.Location` (`GameplayStatics.BreakHitResult` (`self.GetHitResultUnderCursorByChannel` "TraceTypeQuery1"))))))

(fn `UpdateCameraPosition`
  (`/Engine/EditorBlueprintResources/StandardMacros.IsValid` (`self.ServerCharacter`)
    (:`Is Valid`
      (`self.K2_SetActorLocation` (`self.K2_GetPawn`) (`KismetMathLibrary.VInterpTo` (`self.K2_GetActorLocation` (`self.K2_GetPawn`)) (`self.K2_GetActorLocation` (`self.ServerCharacter`)) (`GameplayStatics.GetWorldDeltaSeconds`) (`self.CameraInterpSpeed`)) false false))))

(fn `UserConstructionScript`)