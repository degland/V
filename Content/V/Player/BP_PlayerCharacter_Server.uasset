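; Player character Blueprint that lets other sources take over the camera and block player movement.
; Camera overrides blend the view target to a new source, and release blends back to the controlled pawn if the caller matches the stored source.
; Blocking movement stops the controller, then a client event records the source and sets BlockMovement on BP_PlayerController_Client.
; Releasing movement clears that flag after a source comparison.
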(event `OverrideCamera`
  (params (NewCameraSource :type "Actor Object Reference") (BlendTime :type "Float (double-precision)" :default 1.0))
  ;[1 1 1] Override camera
  (bind _output_get (set `self.CameraOverrideSource` NewCameraSource))
  (`PlayerController.SetViewTargetWithBlend` (`GameplayStatics.GetPlayerController` 0) _output_get BlendTime "VTBlend_Linear" 0.0 false))

(event `ReleaseCamera`
  (params (CameraSource :type "Actor Object Reference"))
  (bind _returnvalue (`GameplayStatics.GetPlayerController` 0))
  ;[1 1 1] Override camera
  (if (== CameraSource (`self.CameraOverrideSource`))
    (`PlayerController.SetViewTargetWithBlend` _returnvalue (`Controller.K2_GetPawn` _returnvalue) 1.0 "VTBlend_Linear" 0.0 false)
    (set `self.CameraOverrideSource` null)))

(event `BlockMovement`
  (params (MovementBlockSource :type "Actor Object Reference"))
  ;[1 1 1] Block movement
  (`Controller.StopMovement` (`self.GetController`))
  (`self.BlockMovementClient` MovementBlockSource))

(event `BlockMovementClient`
  (params (MovementBlockSource :type "Actor Object Reference"))
  ;[1 1 1] Block movement
  (set `self.MovementBlockSource` MovementBlockSource)
  (bind _asbp_player_controller_client (cast `/Game/V/Player/BP_PlayerController_Client` (`GameplayStatics.GetPlayerController` 0)))
  (set `/Game/V/Player/BP_PlayerController_Client.BlockMovement` true _asbp_player_controller_client))

(event `ReleaseMovement`
  (params (MovementBlockSource :type "Actor Object Reference"))
  ;[1 1 1] Block movement
  (if (== MovementBlockSource (`self.MovementBlockSource`))
    (set `self.MovementBlockSource` null)
    (bind _asbp_player_controller_client (cast `/Game/V/Player/BP_PlayerController_Client` (`GameplayStatics.GetPlayerController` 0)))
    (set `/Game/V/Player/BP_PlayerController_Client.BlockMovement` false _asbp_player_controller_client)))

(fn `UserConstructionScript`)