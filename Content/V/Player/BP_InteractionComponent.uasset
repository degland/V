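; Player interaction component that tracks a single current interact target and toggles its on-screen prompt.
; Registering accepts only targets implementing BPI_Interact and shows the given prompt, while unregistering clears and hides it only if that target is still current.
; DoInteract forwards an interact message to the stored target, passing the owning BP_PlayerCharacter_Server cached at BeginPlay.
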(event `self.ReceiveBeginPlay`
  (bind _asbp_player_character_server (cast `/Game/V/Player/BP_PlayerCharacter_Server` (`self.GetOwner`)))
  (set `self.ServerCharacter` _asbp_player_character_server))

(event `RegisterInteractTarget`
  (params (NewTarget :type "Actor Object Reference") (InteractPrompt :type "WidgetComponent Object Reference"))
  (if (`KismetSystemLibrary.DoesImplementInterface` NewTarget "/Game/V/Payload/BPI_Interact.BPI_Interact_C")
    (set `self.InteractTarget` NewTarget)
    (`self.ToggleInteractPrompt` InteractPrompt true)))

(event `UnregisterInteractTarget`
  (params (RemoveTarget :type "Actor Object Reference") (InteractPrompt :type "WidgetComponent Object Reference"))
  (if (== (`self.InteractTarget`) RemoveTarget)
    (set `self.InteractTarget` null)
    (`self.ToggleInteractPrompt` InteractPrompt)))

(event `DoInteract`
  (bind _interacttarget (`self.InteractTarget`))
  (`/Engine/EditorBlueprintResources/StandardMacros.IsValid` _interacttarget
    (:`Is Valid`
      (message `/Game/V/Payload/BPI_Interact.Receive Interact` _interacttarget (`self.ServerCharacter`)))))

(event `ToggleInteractPrompt`
  (params (Prompt :type "WidgetComponent Object Reference") (NewVisibility :type Boolean))
  (`/Engine/EditorBlueprintResources/StandardMacros.IsValid` Prompt
    (:`Is Valid`
      (`SceneComponent.SetVisibility` Prompt NewVisibility true))
    (:`Is Not Valid`
      (`KismetSystemLibrary.PrintString` "invalid interact prompt"))))